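; BP_Enemy is an enemy that travels along a referenced spline and can be killed for gold.
; Tick advances a distance by Speed and places the actor at that point on the spline, matching its rotation.
; TakeDamage lowers Health; at zero or below, only when both DamageDealerSide and ArenaSide are 1, it pays GoldReward to BP_Player and destroys the enemy.
; The fallback destroy branch is unreachable behind a constant-true condition.
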(event EventBeginPlay)

(event Collision|EventActorBeginOverlap
  (params (OtherActor :type Actor%20Object%20Reference)))

(event EventTick
  (params (DeltaSeconds :type Float%20%28single-precision%29))
  (bind _splineref (Variables|Default|GetSplineRef))
  (bind _spline (Variables|/Game/Blueprint/BP_Path.BP_Path_C|GetSpline _splineref))
  (bind _output_get (Variables|Default|SetDistance (+ (Variables|Default|GetDistance) (* DeltaSeconds (Variables|Default|GetSpeed)))))
  (Transformation|SetActorLocation (Spline|GetLocationatDistanceAlongSpline _spline _output_get "World") false false)
  (Transformation|SetActorRotation (Spline|GetRotationatDistanceAlongSpline _spline _output_get "World")))

(fn ConstructionScript)

(fn TakeDamage
  (params (Damage :type Float%20%28double-precision%29) (DamageDealerSide :type Integer))
  (Variables|Default|SetHealth (- (Variables|Default|GetHealth) Damage))
  (if (<= (Variables|Default|GetHealth) 0.0)
    (if true
      (if (and (== DamageDealerSide 1) (== (Variables|Default|GetArenaSide) 1))
        (bind _asbp_player (Utilities|Casting|CastToBP_Player (Game|Player|GetPlayerPawn 0)))
        (Default|AddCoins _asbp_player (Variables|Default|GetGoldReward))
        (Actor|DestroyActor))
      (else
        (Actor|DestroyActor)))))