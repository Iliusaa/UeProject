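; Enemy opponent manager that holds the enemy's coins and base health and automatically builds towers on side 2 tower spots.
; Gathers those spots on BeginPlay, builds starting towers, then attempts another on a looping timer.
; Each attempt picks a random spot and tower type (Base, Mage, Saw), skipping if occupied or unaffordable; costs are hardcoded, bypassing GetTowerCost.
; AddCoins funds building, and TakeBaseDamage shows the player's win result at zero health.
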(event Custom|TryBuildTower
  (CallFunction|BuildRandomEnemyTowers 1))

(event EventBeginPlay
  (bind _outactors (Actor|GetAllActorsOfClass "/Game/Blueprint/BP_TowerSpot.BP_TowerSpot_C"))
  (for _array_element _outactors
    (bind _asbp_tower_spot (Utilities|Casting|CastToBP_TowerSpot _array_element))
    (if (== (Variables|/Game/Blueprint/BP_TowerSpot.BP_TowerSpot_C|GetSpotSide _asbp_tower_spot) 2)
      (Utilities|Array|Add (Variables|Default|GetEnemyTowerSpots) _asbp_tower_spot)))
  (CallFunction|BuildRandomEnemyTowers (Variables|Default|GetStartingTowerCount))
  (Utilities|Time|SetTimerbyEvent (delegate Custom|TryBuildTower) 1e+01 true))

(event Collision|EventActorBeginOverlap
  (params (OtherActor :type Actor%20Object%20Reference)))

(event EventTick
  (params (DeltaSeconds :type Float%20%28single-precision%29)))

(fn ConstructionScript)

(fn BuildRandomEnemyTowers
  (params (Count :type Integer))
  (bind _enemytowerspots (Variables|Default|GetEnemyTowerSpots))
  (for _index (range 0 (- Count 1))
    (if (> (Utilities|Array|Length (Variables|Default|GetEnemyTowerSpots)) 0)
      (bind _output_get (Variables|Default|SetSelectedSpot (Utilities|Array|Get(acopy) _enemytowerspots (Math|Random|RandomIntegerinRange 0 (- (Utilities|Array|Length _enemytowerspots) 1)))))
      (if (not (Variables|/Game/Blueprint/BP_TowerSpot.BP_TowerSpot_C|GetbIsOccupied _output_get))
        (switch int (Math|Random|RandomIntegerinRange 1 3)
          (:1
            (if (>= (Variables|Default|GetEnemyCoins) 25)
              (Variables|Default|SetEnemyCoins (- (Variables|Default|GetEnemyCoins) 25))
              (bind _returnvalue (Game|SpawnActorfromClass "/Game/Blueprint/BP_Tower_Base.BP_Tower_Base_C" (Transformation|GetActorTransform (Variables|Default|GetSelectedSpot)) "Undefined" "MultiplyWithRoot" 0 0))
              (Variables|/Game/Blueprint/BP_Tower_Base.BP_Tower_Base_C|SetTowerSide _returnvalue 2)
              (Variables|/Game/Blueprint/BP_TowerSpot.BP_TowerSpot_C|SetbIsOccupied (Variables|Default|GetSelectedSpot) true)))
          (:2
            (if (>= (Variables|Default|GetEnemyCoins) 50)
              (Variables|Default|SetEnemyCoins (- (Variables|Default|GetEnemyCoins) 50))
              (bind _returnvalue_2 (Game|SpawnActorfromClass "/Game/Blueprint/BP_Tower_Mage.BP_Tower_Mage_C" (Transformation|GetActorTransform (Variables|Default|GetSelectedSpot)) "Undefined" "MultiplyWithRoot" 0 0))
              (Variables|/Game/Blueprint/BP_Tower_Base.BP_Tower_Base_C|SetTowerSide _returnvalue_2 2)
              (Variables|/Game/Blueprint/BP_TowerSpot.BP_TowerSpot_C|SetbIsOccupied (Variables|Default|GetSelectedSpot) true)))
          (:3
            (if (>= (Variables|Default|GetEnemyCoins) 40)
              (Variables|Default|SetEnemyCoins (- (Variables|Default|GetEnemyCoins) 45))
              (bind _returnvalue_3 (Game|SpawnActorfromClass "/Game/Blueprint/BP_Tower_Saw.BP_Tower_Saw_C" (Transformation|GetActorTransform (Variables|Default|GetSelectedSpot)) "Undefined" "MultiplyWithRoot" 0 0))
              (Variables|/Game/Blueprint/BP_Tower_Base.BP_Tower_Base_C|SetTowerSide _returnvalue_3 2)
              (Variables|/Game/Blueprint/BP_TowerSpot.BP_TowerSpot_C|SetbIsOccupied (Variables|Default|GetSelectedSpot) true))))))))

(fn AddCoins
  (params (amount :type Integer))
  (Variables|Default|SetEnemyCoins (+ (Variables|Default|GetEnemyCoins) amount)))

(fn GetTowerCost
  (params (TowerType :type Integer))
  (switch int TowerType
    (:Default
      (return 999999))
    (:1
      (return 25))
    (:2
      (return 50))
    (:3
      (return 45))))

(fn TakeBaseDamage
  (params (Damage :type Integer))
  (Variables|Default|SetEnemyHealth (- (Variables|Default|GetEnemyHealth) Damage))
  (if (<= (Variables|Default|GetEnemyHealth) 0)
    (bind _asbp_player (Utilities|Casting|CastToBP_Player (Game|GetPlayerCharacter 0)))
    (Default|ShowGameResult _asbp_player true)))