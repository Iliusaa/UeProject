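; Player character for a tower-building game, with first-person-style movement, look and jump, plus a coin balance.
; Each tick a camera line trace stores the tower spot under the view, and input actions select an archer, mage or saw tower.
; Pressing E on an unoccupied side-1 spot spends the hardcoded cost, spawns the selected tower there on side 1, and marks the spot occupied.
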(event EventBeginPlay)

(event Collision|EventActorBeginOverlap
  (params (OtherActor :type Actor%20Object%20Reference)))

(event EventTick
  (params (DeltaSeconds :type Float%20%28single-precision%29))
  ;[0.15 0.15 0.15 0.5] camera beamcast
  (bind _outhit (Collision|LineTraceByChannel (Transformation|GetWorldLocation (Variables|Default|GetCamera)) (+ (Transformation|GetWorldLocation (Variables|Default|GetCamera)) (* (Math|Vector|GetForwardVector (Variables|Default|GetCamera)) (Math|Conversions|ToFloat(Integer) 5000))) "TraceTypeQuery1" false 0 "None"))
  (bind _asbp_tower_spot (Utilities|Casting|CastToBP_TowerSpot (.HitActor (Collision|BreakHitResult _outhit)))
    (:then
      (Variables|Default|SetCurrentTowerSpot _asbp_tower_spot))
    (:CastFailed
      (Variables|Default|SetCurrentTowerSpot 0))))

(event Input|ActionEvents|InputActionJump
  (params (Key :type Key%20Structure :default "None"))
  ;[0.15 0.15 0.15 0.5] movement
  (:Pressed
    (Character|Jump))
  (:Released
    (Character|StopJumping)))

(event Input|ActionEvents|InputActionSelectTower_Archer
  (params (Key :type Key%20Structure :default "None"))
  ;[0.15 0.15 0.15 0.5] selection archer/mage/saw
  (:Pressed
    (Variables|Default|SetSelectedTowerType 1))
  (:Released
    (Development|PrintString "archer")))

(event Input|ActionEvents|InputActionSelectTower_Mage
  (params (Key :type Key%20Structure :default "None"))
  ;[0.15 0.15 0.15 0.5] selection archer/mage/saw
  (:Pressed
    (Variables|Default|SetSelectedTowerType 2))
  (:Released
    (Development|PrintString "mage")))

(event Input|ActionEvents|InputActionSelectTower_Saw
  (params (Key :type Key%20Structure :default "None"))
  ;[0.15 0.15 0.15 0.5] selection archer/mage/saw
  (:Pressed
    (Variables|Default|SetSelectedTowerType 3))
  (:Released
    (Development|PrintString "saw")))

(event Input|AxisEvents|InputAxisMoveForward
  (params (AxisValue :type Float%20%28single-precision%29))
  ;[0.15 0.15 0.15 0.5] movement
  (Pawn|Input|AddMovementInput (Math|Vector|GetForwardVector (Math|Rotator|MakeRotator 0.0 0.0 (.Yaw (Math|Rotator|BreakRotator (Pawn|GetControlRotation (Pawn|GetController) :!class /Script/Engine.Controller))))) AxisValue false))

(event Input|AxisEvents|InputAxisMoveRight
  (params (AxisValue :type Float%20%28single-precision%29))
  ;[0.15 0.15 0.15 0.5] movement
  (Pawn|Input|AddMovementInput (Math|Vector|GetRightVector (Variables|Default|GetCamera)) AxisValue false))

(event Input|AxisEvents|InputAxisTurn
  (params (AxisValue :type Float%20%28single-precision%29))
  ;[0.15 0.15 0.15 0.5] movement
  (Pawn|Input|AddControllerYawInput AxisValue))

(event Input|AxisEvents|InputAxisLookUp
  (params (AxisValue :type Float%20%28single-precision%29))
  ;[0.15 0.15 0.15 0.5] movement
  (Pawn|Input|AddControllerPitchInput AxisValue))

(event Input|KeyboardEvents|E
  (params (Key :type Key%20Structure :default "None"))
  (bind _currenttowerspot (Variables|Default|GetCurrentTowerSpot))
  (bind _returnvalue (Transformation|GetActorLocation _currenttowerspot))
  (bind _returnvalue_2 (Math|Transform|MakeTransform _returnvalue))
  ;[0.15 0.15 0.15 0.5] e key logic
  (:Pressed
    (Utilities|IsValid (Variables|Default|GetCurrentTowerSpot)
      (:Is%20Valid
        (if (== (Variables|/Game/Blueprint/BP_TowerSpot.BP_TowerSpot_C|GetSpotSide (Variables|Default|GetCurrentTowerSpot)) 1)
          (if (not (Variables|/Game/Blueprint/BP_TowerSpot.BP_TowerSpot_C|GetbIsOccupied (Variables|Default|GetCurrentTowerSpot)))
            (bind _cost (CallFunction|GetSelectedTowerCost))
            (bind _canspend (CallFunction|TrySpendCoins _cost))
            (if _canspend
              (switch int (Variables|Default|GetSelectedTowerType)
                (:1
                  (bind _returnvalue_3 (Game|SpawnActorfromClass "/Game/Blueprint/BP_Tower_Base.BP_Tower_Base_C" _returnvalue_2 "Undefined" "MultiplyWithRoot" 0 0))
                  (Variables|/Game/Blueprint/BP_Tower_Base.BP_Tower_Base_C|SetTowerSide _returnvalue_3 1))
                (:2
                  (bind _returnvalue_4 (Game|SpawnActorfromClass "/Game/Blueprint/BP_Tower_Mage.BP_Tower_Mage_C" _returnvalue_2 "Undefined" "MultiplyWithRoot" 0 0))
                  (Variables|/Game/Blueprint/BP_Tower_Base.BP_Tower_Base_C|SetTowerSide _returnvalue_4 1))
                (:3
                  (bind _returnvalue_5 (Game|SpawnActorfromClass "/Game/Blueprint/BP_Tower_Saw.BP_Tower_Saw_C" _returnvalue_2 "Undefined" "MultiplyWithRoot" 0 0))
                  (Variables|/Game/Blueprint/BP_Tower_Base.BP_Tower_Base_C|SetTowerSide _returnvalue_5 1)))
              (Variables|/Game/Blueprint/BP_TowerSpot.BP_TowerSpot_C|SetbIsOccupied (Variables|Default|GetCurrentTowerSpot) true))))))))

(fn ConstructionScript)

(fn AddCoins
  (params (Amount :type Integer))
  (bind _output_get (Variables|Default|SetCoins (+ Amount (Variables|Default|GetCoins)))))

(fn TrySpendCoins
  (params (Cost :type Integer))
  (if (>= (Variables|Default|GetCoins) Cost)
    (Variables|Default|SetCoins (- (Variables|Default|GetCoins) Cost))
    (return true)
    (else
      (Development|PrintString "not enough coins")
      (return false))))

(fn GetSelectedTowerCost
  (switch int (Variables|Default|GetSelectedTowerType)
    (:Default
      (return 999999))
    (:1
      (return 25))
    (:2
      (return 50))
    (:3
      (return 45))))