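; BP_Spawner is an actor that periodically spawns random enemies at its spawn point.
; On BeginPlay a looping timer set by SpawnDelay fires SpawnEnemy, which picks a random class from EnemyClasses, provided the array is not empty.
; Each spawned actor gets ArenaSide 1, and those that are BP_Enemy receive the spawner's SplineRef.
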(event Custom|SpawnEnemy
  (bind _enemyclasses (Variables|Default|GetEnemyClasses))
  (bind _returnvalue (Utilities|Array|Length _enemyclasses))
  (if (> _returnvalue 0)
    (bind _returnvalue_2 (Game|SpawnActorfromClass (Utilities|Array|Get(acopy) (Variables|Default|GetEnemyClasses) (Math|Random|RandomIntegerinRange 0 (- _returnvalue 1))) (Math|Transform|MakeTransform (Transformation|GetWorldLocation (Variables|Default|GetSpawnPoint))) "Undefined" "MultiplyWithRoot" 0 0))
    (Variables|/Game/Blueprint/BP_Enemy.BP_Enemy_C|SetArenaSide _returnvalue_2 1)
    (bind _asbp_enemy (Utilities|Casting|CastToBP_Enemy _returnvalue_2))
    (Variables|/Game/Blueprint/BP_Enemy.BP_Enemy_C|SetSplineRef _asbp_enemy (Variables|Default|GetSplineRef))))

(event EventBeginPlay
  (Utilities|Time|SetTimerbyEvent (delegate Custom|SpawnEnemy) (Variables|Default|GetSpawnDelay) true))

(event Collision|EventActorBeginOverlap
  (params (OtherActor :type Actor%20Object%20Reference)))

(event EventTick
  (params (DeltaSeconds :type Float%20%28single-precision%29)))

(fn ConstructionScript)