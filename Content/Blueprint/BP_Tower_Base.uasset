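; BP_Tower_Base is a defensive tower that automatically shoots arrows at enemies whose ArenaSide matches its TowerSide.
; The Range sphere's overlap events maintain an EnemiesInRange list, and Tick targets the first entry.
; Each tick yaws the Pivot toward that target with a 90-degree offset.
; When CanShoot allows, it spawns an aimed BP_ArrowProjectile tagged with TowerSide, then waits FireRate via Delay before re-arming.
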(event OnComponentBeginOverlap(Range)
  (params (OverlappedComponent :type Primitive%20Component%20Object%20Reference) (OtherActor :type Actor%20Object%20Reference) (OtherComp :type Primitive%20Component%20Object%20Reference) (OtherBodyIndex :type Integer) (bFromSweep :type Boolean) (SweepResult :type Hit%20Result%20Structure%20%28by%20ref%29))
  (bind _asbp_enemy (Utilities|Casting|CastToBP_Enemy OtherActor))
  (if (== (Variables|/Game/Blueprint/BP_Enemy.BP_Enemy_C|GetArenaSide _asbp_enemy) (Variables|Default|GetTowerSide))
    (Utilities|Array|AddUnique (Variables|Default|GetEnemiesInRange) _asbp_enemy)))

(event OnComponentEndOverlap(Range)
  (params (OverlappedComponent :type Primitive%20Component%20Object%20Reference) (OtherActor :type Actor%20Object%20Reference) (OtherComp :type Primitive%20Component%20Object%20Reference) (OtherBodyIndex :type Integer))
  ;[0.15 0.15 0.15 0.5] check if enemy is real
  (bind _asbp_enemy (Utilities|Casting|CastToBP_Enemy OtherActor))
  (Utilities|Array|RemoveItem (Variables|Default|GetEnemiesInRange) _asbp_enemy))

(event EventTick
  (params (DeltaSeconds :type Float%20%28single-precision%29))
  (if (> (Utilities|Array|Length (Variables|Default|GetEnemiesInRange)) 0)
    (bind _output_get (Variables|Default|SetTargetEnemy (Utilities|Array|Get(acopy) (Variables|Default|GetEnemiesInRange))))
    (Utilities|IsValid _output_get :!label _label
      (:Is%20Valid
        (Transformation|SetRelativeRotation (Variables|Default|GetPivot) (Math|Rotator|MakeRotator 0.0 0.0 (+ (.Yaw (Math|Rotator|BreakRotator (Math|Rotator|FindLookatRotation (Transformation|GetWorldLocation (Variables|Default|GetPivot)) (Transformation|GetActorLocation (Variables|Default|GetTargetEnemy))))) 9e+01)) false false)
        ;[0.15 0.15 0.15 0.5] spawn logic + spawn position
        (if (Variables|Default|GetCanShoot)
          (bind _returnvalue (Game|SpawnActorfromClass "/Game/Blueprint/BP_ArrowProjectile.BP_ArrowProjectile_C" (Math|Transform|MakeTransform (Transformation|GetWorldLocation (Variables|Default|GetArrowSpawnPoint)) (Math|Rotator|FindLookatRotation (Transformation|GetWorldLocation (Variables|Default|GetArrowSpawnPoint)) (+ (Transformation|GetActorLocation (Variables|Default|GetTargetEnemy)) "0.000000,0.000000,5.000000")) "5.000000,5.000000,5.000000") "Undefined" "MultiplyWithRoot" 0 0))
          (Variables|/Game/Blueprint/BP_ArrowProjectile.BP_ArrowProjectile_C|SetProjectileSide _returnvalue (Variables|Default|GetTowerSide))
          (Variables|Default|SetCanShoot false)
          (Utilities|FlowControl|Delay (Variables|Default|GetFireRate))
          (Variables|Default|SetCanShoot true)
          (goto _label)))
      (:Is%20Not%20Valid
        (Variables|Default|SetTargetEnemy 0)))))

(fn ConstructionScript)