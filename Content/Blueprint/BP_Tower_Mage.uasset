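; BP_Tower_Mage is a tower that attacks BP_Enemy actors whose arena side matches its own.
; Its Range overlap collects those enemies, and Tick targets the first array entry, with no removal logic here.
; Each shot applies instant damage and spawns an ice-trail Niagara beam between tower and target.
; A CanShoot gate and FireRate delay pace fire, then destroy the beam and re-enter the shot logic.
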(event OnComponentBeginOverlap(Range)
  (params (OverlappedComponent :type Primitive%20Component%20Object%20Reference) (OtherActor :type Actor%20Object%20Reference) (OtherComp :type Primitive%20Component%20Object%20Reference) (OtherBodyIndex :type Integer) (bFromSweep :type Boolean) (SweepResult :type Hit%20Result%20Structure%20%28by%20ref%29))
  (bind _asbp_enemy (Utilities|Casting|CastToBP_Enemy OtherActor))
  (if (== (Variables|/Game/Blueprint/BP_Enemy.BP_Enemy_C|GetArenaSide _asbp_enemy) (Variables|Default|GetTowerSide))
    (Utilities|Array|AddUnique (Variables|Default|GetEnemiesInRange) _asbp_enemy)))

(event EventBeginPlay
  (|CallParentFunction) ; This node is disabled and will not be called.\nDrag off pins to build functionality.
)

(event Collision|EventActorBeginOverlap
  (params (OtherActor :type Actor%20Object%20Reference))
  (|CallParentFunction OtherActor) ; This node is disabled and will not be called.\nDrag off pins to build functionality.
)

(event EventTick
  (params (DeltaSeconds :type Float%20%28single-precision%29))
  (bind _beamspawnpoint (Variables|Default|GetBeamSpawnPoint))
  (if (> (Utilities|Array|Length (Variables|Default|GetEnemiesInRange)) 0)
    (bind _output_get (Variables|Default|SetTargetEnemy (Utilities|Array|Get(acopy) (Variables|Default|GetEnemiesInRange))))
    (Utilities|IsValid _output_get :!label _label
      (:Is%20Valid
        (Utilities|FlowControl|Sequence
          (:then_0
            ;[0.15 0.15 0.15 0.5] spawn logic + spawn position
            (if (Variables|Default|GetCanShoot)
              (Collision|LineTraceByChannel (Transformation|GetWorldLocation (Variables|Default|GetBeamSpawnPoint)) (Transformation|GetActorLocation (Variables|Default|GetTargetEnemy)) "TraceTypeQuery1" false 0 "None")
              (bind _returnvalue (Niagara|SpawnSystemAttached "/Game/ArrowTrail/FX/NS_ArrowTrail_Ice.NS_ArrowTrail_Ice" _beamspawnpoint "None" "0, 0, 0" "0, 0, 0" "KeepRelativeOffset" true))
              (Niagara|SetNiagaraVariable(Vector3) _returnvalue "User.Start" (Transformation|GetWorldLocation _beamspawnpoint))
              (Niagara|SetNiagaraVariable(Vector3) _returnvalue "User.End" (Transformation|GetActorLocation (Variables|Default|GetTargetEnemy)))
              (Default|TakeDamage (Variables|Default|GetTargetEnemy) (Variables|Default|GetDamage) (Variables|Default|GetTowerSide))
              (Variables|Default|SetCanShoot false)
              (Utilities|FlowControl|Delay (Variables|Default|GetFireRate))
              (bind _output_get_2 (Variables|Default|SetBeamNiagaraRef _returnvalue))
              (Components|DestroyComponent _output_get_2)
              (Variables|Default|SetCanShoot true)
              (goto _label)))))
      (:Is%20Not%20Valid
        (Variables|Default|SetTargetEnemy 0)))))

(fn ConstructionScript
  (|CallParentFunction))